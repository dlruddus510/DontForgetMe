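; BP_Bomb is a homing bomb pawn, filed under BossCreeper, that chases a player and explodes.
; Two PawnSensing components each trigger an AI MoveTo toward a fixed target, player 0's BearCharacter or player 1's Robot, regardless of which pawn was seen.
; Reaching the target destroys the bomb, spawns an explosion and damages that character.
; A failed move explodes it without damage after a delay, longer for the Robot.
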(event OnSeePawn(PawnSensing)
  (params (Pawn :type Pawn%20Object%20Reference))
  (Variables|Default|SetisSeeingPlayer? true)
  (CallFunction|FollowPlayer))

(event OnSeePawn(PawnSensing1)
  (params (Pawn :type Pawn%20Object%20Reference))
  (Variables|Default|SetisSeeingPlayer? true)
  (CallFunction|FollowRobot))

(event Custom|FollowPlayer
  (bind _asbear_character (Utilities|Casting|CastToBearCharacter (Game|GetPlayerCharacter 0)))
  (if (Variables|Default|GetisSeeingPlayer?)
    (AI|AIMoveTo self "0, 0, 0" _asbear_character 5.0 false
      (:OnSuccess
        (Actor|DestroyActor)
        (Effects|SpawnEmitteratLocation "/Game/FXVarietyPack/Particles/P_ky_explosion.P_ky_explosion" (Transformation|GetActorLocation))
        (Utilities|IsValid _asbear_character
          (:Is%20Valid
            (Class|ITTCharacter|TakeDamage _asbear_character 0.0 (Utilities|Struct|MakeDamageEvent)))))
      (:OnFail
        (Utilities|FlowControl|Delay 1.0)
        (Actor|DestroyActor)
        (Effects|SpawnEmitteratLocation "/Game/FXVarietyPack/Particles/P_ky_explosion.P_ky_explosion" (Transformation|GetActorLocation))))))

(event Custom|FollowRobot
  (bind _asrobot (Utilities|Casting|CastToRobot (Game|GetPlayerCharacter 1)))
  (if (Variables|Default|GetisSeeingPlayer?)
    (AI|AIMoveTo self "0, 0, 0" _asrobot 5.0 false
      (:OnSuccess
        (Actor|DestroyActor)
        (Effects|SpawnEmitteratLocation "/Game/FXVarietyPack/Particles/P_ky_explosion.P_ky_explosion" (Transformation|GetActorLocation))
        (Utilities|IsValid _asrobot
          (:Is%20Valid
            (Class|ITTCharacter|TakeDamage _asrobot 0.0 (Utilities|Struct|MakeDamageEvent)))))
      (:OnFail
        (Utilities|FlowControl|Delay 6.0)
        (Actor|DestroyActor)
        (Effects|SpawnEmitteratLocation "/Game/FXVarietyPack/Particles/P_ky_explosion.P_ky_explosion" (Transformation|GetActorLocation))))))

(fn ConstructionScript)