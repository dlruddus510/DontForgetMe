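; Boss bomb spawner for the creeper boss that drops bombs at random reachable navmesh points around itself.
; A looping one-second timer spawns BP_Bomb, or BP_FailBomb about a quarter of the time, within a wide radius.
; A four-spawn cap is meant to clear the timer, but each spawn resets TotalSpawnCount before incrementing, so the cap is never reached.
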(event Custom|Spawn%20Enemy
  (bind _returnvalue (Transformation|GetActorLocation))
  (bind _randomlocation (AI|Navigation|GetRandomReachablePointinRadius _returnvalue 7e+03 0 0))
  (if (< (Variables|Default|GetTotalSpawnCount) 4)
    (if (Math|Conversions|ToBoolean(Integer) (Math|Random|RandomIntegerinRange 0 3))
      (Game|SpawnActorfromClass "/Game/BossCreeper/BP_Bomb.BP_Bomb_C" (Math|Transform|MakeTransform _randomlocation "0, 0, 0" "1.000000,1.000000,1.000000") "Undefined" 0 0)
      (Variables|Default|SetFailedBombIndex true)
      (bind _output_get (Variables|Default|SetTotalSpawnCount 0))
      (Math|Integer|IncrementInt _output_get)
      (else
        (Game|SpawnActorfromClass "/Game/BossCreeper/BP_FailBomb.BP_FailBomb_C" (Math|Transform|MakeTransform _randomlocation "0, 0, 0" "1.000000,1.000000,1.000000") "Undefined" 0 0)
        (bind _output_get_2 (Variables|Default|SetTotalSpawnCount 0))
        (Math|Integer|IncrementInt _output_get_2
          (:%20%20
            (Development|PrintString "failed")))))
    (else
      (Utilities|Time|ClearTimerbyFunctionName 0 "\"Spawn Enemy\""))))

(event EventBeginPlay
  (Utilities|Time|SetTimerbyEvent (delegate Custom|Spawn%20Enemy) 1.0 true))

(fn ConstructionScript)