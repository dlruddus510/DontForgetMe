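; BP_FailBomb is a bomb actor in the BossCreeper folder that explodes with a particle effect and destroys itself.
; It detonates 60 seconds after BeginPlay, or when BombDestroy is called.
; Two PawnSensing components set IsSeeingPlayer and call FollowPlayer or FollowRobot, but both events are empty.
; Chase and damage logic for BearCharacter and Robot is left disconnected, so the bomb deals no damage itself.
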(event OnActorBeginOverlap(BossHit)
  (params (OverlappedActor :type Actor%20Object%20Reference) (OtherActor :type Actor%20Object%20Reference)))

(event OnSeePawn(PawnSensing)
  (params (Pawn :type Pawn%20Object%20Reference))
  (Variables|Default|SetisSeeingPlayer? true)
  (CallFunction|FollowPlayer))

(event OnComponentHit(StaticMesh)
  (params (HitComponent :type Primitive%20Component%20Object%20Reference) (OtherActor :type Actor%20Object%20Reference) (OtherComp :type Primitive%20Component%20Object%20Reference) (NormalImpulse :type Vector :default "0, 0, 0") (Hit :type Hit%20Result%20Structure%20%28by%20ref%29)))

(event OnSeePawn(PawnSensing1)
  (params (Pawn :type Pawn%20Object%20Reference))
  (Variables|Default|SetisSeeingPlayer? true)
  (CallFunction|FollowRobot))

(event Custom|BombDestroy
  (Effects|SpawnEmitteratLocation "/Game/FXVarietyPack/Particles/P_ky_explosion.P_ky_explosion" (Transformation|GetActorLocation))
  (Actor|DestroyActor))

(event Custom|FollowPlayer)

(event Custom|FollowRobot)

(event Collision|EventActorBeginOverlap
  (params (OtherActor :type Actor%20Object%20Reference)))

(event EventBeginPlay
  (Utilities|FlowControl|Delay 6e+01)
  (Actor|DestroyActor)
  (Effects|SpawnEmitteratLocation "/Game/FXVarietyPack/Particles/P_ky_explosion.P_ky_explosion" (Transformation|GetActorLocation)))

(fn ConstructionScript)