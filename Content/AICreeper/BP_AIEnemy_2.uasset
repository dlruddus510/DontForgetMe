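; BP_AIEnemy_2 is an AI enemy pawn meant to chase the player when it sees one.
; Its PawnSensing sight event casts the player character to BP_AIEnemy and runs AI MoveTo toward it only if that cast succeeds.
; A FollowPlayer event moves to the player while IsSeeingPlayer is true, but the nodes that set the flag and call it are disconnected.
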(event OnSeePawn(PawnSensing)
  (params (Pawn :type Pawn%20Object%20Reference))
  (bind _asbp_aienemy (Utilities|Casting|CastToBP_AIEnemy (Game|GetPlayerCharacter 0)))
  (AI|AIMoveTo self "0, 0, 0" _asbp_aienemy 5.0 false))

(event Custom|FollowPlayer
  (if (Variables|Default|GetisSeeingPlayer?)
    (AI|AIMoveTo self "0, 0, 0" (Game|GetPlayerCharacter 0) 5.0 false)))

(event EventBeginPlay)

(event Collision|EventActorBeginOverlap
  (params (OtherActor :type Actor%20Object%20Reference)))

(event EventTick
  (params (DeltaSeconds :type Float%20%28single-precision%29)))

(fn ConstructionScript)