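; BP_PuzzleBoard is a tangram puzzle board that snaps a released piece onto its own location and rotation.
; Actor overlap begin and end switch its Tick on and off.
; While ticking, it casts the last overlapping actor to BP_Master_Grab_Child and snaps it once the player is not controlling it and its PuzzleBlock reports IsInPlace.
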(event EventBeginPlay)

(event Collision|EventActorBeginOverlap
  (params (OtherActor :type Actor%20Object%20Reference))
  (Actor|Tick|SetActorTickEnabled true))

(event EventTick
  (params (DeltaSeconds :type Float%20%28single-precision%29))
  (bind _asbp_master_grab_child (Utilities|Casting|CastToBP_Master_Grab_Child (stale Collision|EventActorBeginOverlap OtherActor)))
  (if (and (not (Variables|/Game/GrabSystem/Blueprint/Actor/BP_Master_Grab.BP_Master_Grab_C|GetControllingByPlayer _asbp_master_grab_child)) (Class|PuzzleBlockComponent|IsinPlace (Variables|/Game/Tangram/BP_Master_Grab_Child.BP_Master_Grab_Child_C|GetPuzzleBlock _asbp_master_grab_child)))
    (Transformation|SetActorLocationAndRotation (stale Collision|EventActorBeginOverlap OtherActor) (Transformation|GetActorLocation) (Transformation|GetActorRotation))))

(event Collision|EventActorEndOverlap
  (params (OtherActor :type Actor%20Object%20Reference))
  (Actor|Tick|SetActorTickEnabled false))

(fn ConstructionScript)