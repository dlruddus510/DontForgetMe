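; BP_PuzzleSystem is a tangram puzzle checker that decides whether the puzzle boards inside its Box are solved.
; PuzzleCheck loops over overlapping BP_PuzzleBoard actors, copying each IsGoodBlock into AllBoardSuccess, so the last value overwrites earlier ones rather than combining them.
; That result goes to PuzzleSuccess, which only prints a message when true.
; The event graph is empty, so nothing in this Blueprint calls PuzzleCheck.
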(event EventBeginPlay)

(event Collision|EventActorBeginOverlap
  (params (OtherActor :type Actor%20Object%20Reference)))

(event EventTick
  (params (DeltaSeconds :type Float%20%28single-precision%29)))

(fn ConstructionScript)

(fn PuzzleCheck
  (for _array_element (Collision|GetOverlappingActors (Variables|Default|GetBox) "/Game/Tangram/PuzzleBoard/BP_PuzzleBoard.BP_PuzzleBoard_C" :!class /Script/Engine.PrimitiveComponent)
    (bind _asbp_puzzle_board (Utilities|Casting|CastToBP_PuzzleBoard _array_element))
    (Variables|Default|SetAllBoardSuccess (Variables|/Game/Tangram/PuzzleBoard/BP_PuzzleBoard.BP_PuzzleBoard_C|GetbIsGoodBlock _asbp_puzzle_board)))
  (CallFunction|PuzzleSuccess (Variables|Default|GetAllBoardSuccess)))

(fn PuzzleSuccess
  (params (AllBlockSuccess :type Boolean))
  (if AllBlockSuccess
    (Development|PrintString "PuzzleSuccess")))