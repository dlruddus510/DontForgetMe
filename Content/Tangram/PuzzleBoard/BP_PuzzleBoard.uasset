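; BP_PuzzleBoard is a board slot in the Tangram puzzle that snaps released grab pieces onto its own transform.
; Overlap events switch Tick on and off, so it polls only while an actor is present.
; Tick waits until the piece is no longer player-controlled and its PuzzleBlock reports in place.
; A correctly shaped piece sets IsGoodBlock, calls PuzzleCheck on box-overlapping BP_PuzzleSystem actors and stops ticking.
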(event EventBeginPlay
  (Actor|Tick|SetActorTickEnabled false))

(event Collision|EventActorBeginOverlap
  (params (OtherActor :type Actor%20Object%20Reference))
  (Actor|Tick|SetActorTickEnabled true))

(event EventTick
  (params (DeltaSeconds :type Float%20%28single-precision%29))
  (bind _asbp_master_grab_child (Utilities|Casting|CastToBP_Master_Grab_Child (stale Collision|EventActorBeginOverlap OtherActor)))
  (if (and (not (Variables|/Game/GrabSystem/Blueprint/Actor/BP_Master_Grab.BP_Master_Grab_C|GetControllingByPlayer _asbp_master_grab_child)) (Class|PuzzleBlockComponent|IsinPlace (Variables|/Game/Tangram/PuzzleBlock/BP_Master_Grab_Child.BP_Master_Grab_Child_C|GetPuzzleBlock _asbp_master_grab_child)))
    (Transformation|SetActorLocationAndRotation (stale Collision|EventActorBeginOverlap OtherActor) (Transformation|GetActorLocation) (Transformation|GetActorRotation))
    (if (Class|PuzzleBlockComponent|IsinPlaceandShape (Variables|/Game/Tangram/PuzzleBlock/BP_Master_Grab_Child.BP_Master_Grab_Child_C|GetPuzzleBlock _asbp_master_grab_child))
      (Variables|Default|SetbIsGoodBlock (Class|PuzzleBlockComponent|IsinPlaceandShape (Variables|/Game/Tangram/PuzzleBlock/BP_Master_Grab_Child.BP_Master_Grab_Child_C|GetPuzzleBlock _asbp_master_grab_child)))
      (for _array_element (Collision|GetOverlappingActors (Variables|Default|GetBox) "/Game/Tangram/BP_PuzzleSystem.BP_PuzzleSystem_C" :!class /Script/Engine.PrimitiveComponent)
        (bind _asbp_puzzle_system (Utilities|Casting|CastToBP_PuzzleSystem _array_element))
        (Default|PuzzleCheck _asbp_puzzle_system)
        (Actor|Tick|SetActorTickEnabled false)))))

(event Collision|EventActorEndOverlap
  (params (OtherActor :type Actor%20Object%20Reference))
  (Actor|Tick|SetActorTickEnabled false))

(fn ConstructionScript)