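; Hook projectile that pulls grabbable objects back to the point it was fired from.
; BeginPlay stores the hook's start location, and a hit on anything other than a BP_Master_Grab destroys the hook.
; On a grab hit, two timelines lerp the hook and the target's physics-disabled mesh back to that point, zeroing projectile velocity.
; When the Comeback timeline finishes, it restores the mesh's physics and destroys the hook.
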(event OnComponentHit(hook11)
  (params (HitComponent :type Primitive%20Component%20Object%20Reference) (OtherActor :type Actor%20Object%20Reference) (OtherComp :type Primitive%20Component%20Object%20Reference) (NormalImpulse :type Vector :default "0, 0, 0") (Hit :type Hit%20Result%20Structure%20%28by%20ref%29))
  (bind _asbp_master_grab (Utilities|Casting|CastToBP_Master_Grab OtherActor)
    (:then
      (Variables|Default|SetOtherActor _asbp_master_grab)
      (Utilities|FlowControl|Sequence
        (:then_0
          (bind _새_트랙_0 (Timeline|Comeback PlayFromStart)
            (:Update
              (Variables|/Script/Engine.MovementComponent|SetVelocity (Variables|Default|GetProjectileMovement) "0, 0, 0")
              (Transformation|SetWorldLocation (Variables|Default|Gethook11) (Math|Vector|Lerp(Vector) (Transformation|GetWorldLocation (Variables|Default|Gethook11)) (stale EventBeginPlay _output_get) _새_트랙_0) false false))
            (:Finished
              (Utilities|IsValid (Variables|/Game/GrabSystem/Blueprint/Actor/BP_Master_Grab.BP_Master_Grab_C|GetStaticMesh (Variables|Default|GetOtherActor))
                (:Is%20Valid
                  (Physics|SetSimulatePhysics (Variables|/Game/GrabSystem/Blueprint/Actor/BP_Master_Grab.BP_Master_Grab_C|GetStaticMesh (Variables|Default|GetOtherActor)) true)
                  (Actor|DestroyActor))))))
        (:then_1
          (Physics|SetSimulatePhysics (Variables|/Game/GrabSystem/Blueprint/Actor/BP_Master_Grab.BP_Master_Grab_C|GetStaticMesh _asbp_master_grab) false)
          (bind _새_트랙_0_2 (Timeline|타임라인_0 Play)
            (:Update
              (Transformation|SetWorldLocation (Variables|Default|Gethook11) (Math|Vector|Lerp(Vector) (Transformation|GetWorldLocation (Variables|/Game/GrabSystem/Blueprint/Actor/BP_Master_Grab.BP_Master_Grab_C|GetStaticMesh _asbp_master_grab)) (Variables|Default|GetLocation) _새_트랙_0_2) false false))))))
    (:CastFailed
      (Actor|DestroyActor))))

(event EventBeginPlay
  (bind _output_get (Variables|Default|SetLocation (Transformation|GetWorldLocation (Variables|Default|Gethook11))))
  (Utilities|FlowControl|Delay 0.5))

(event Collision|EventActorBeginOverlap
  (params (OtherActor :type Actor%20Object%20Reference)))

(fn ConstructionScript)