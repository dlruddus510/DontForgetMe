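; BP_Grapple is an actor that handles a grapple hit for the player's BP_Robot.
; On Hit it stores the robot's location and the hit location as the grapple start and end, then calls MoveGrapple on the robot.
; It then polls the robot's movement mode through a very short looping Delay and destroys itself once that mode is None.
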(event Collision|EventHit
  (params (MyComp :type Primitive%20Component%20Object%20Reference) (Other :type Actor%20Object%20Reference) (OtherComp :type Primitive%20Component%20Object%20Reference) (bSelfMoved :type Boolean) (HitLocation :type Vector :default "0, 0, 0") (HitNormal :type Vector :default "0, 0, 0") (NormalImpulse :type Vector :default "0, 0, 0") (Hit :type Hit%20Result%20Structure%20%28by%20ref%29))
  (bind _asbp_robot (Utilities|Casting|CastToBP_Robot (Game|GetPlayerCharacter 0)))
  (Variables|/Game/BP_Character/BP_Robot.BP_Robot_C|SetGrappleStartLoc _asbp_robot (Transformation|GetActorLocation _asbp_robot))
  (Variables|/Game/BP_Character/BP_Robot.BP_Robot_C|SetGrappleEndLoc _asbp_robot HitLocation)
  (Default|MoveGrapple _asbp_robot)
  (Utilities|FlowControl|Delay 0.0001 :!label _label)
  (if (Utilities|Enum|Equal(Enum) (Variables|/Script/Engine.CharacterMovementComponent|GetMovementMode (Variables|/Script/Engine.Character|GetCharacterMovement _asbp_robot)) "MOVE_None")
    (Actor|DestroyActor)
    (else
      (goto _label))))

(fn ConstructionScript)