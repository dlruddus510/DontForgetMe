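; Boss enemy that starts a looping random attack phase and shows its HP bar after an intro delay.
; Every few seconds it swings, spawns a bomb or fail bomb, or drops a hand with a damage area at random spots.
; Left and Right overlaps damage and knock back players.
; An uncontrolled fail bomb entering BoomBox removes all initial health; delayed Tick then plays the death montage and opens EndLevel.
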(event OnComponentBeginOverlap(Right)
  (params (OverlappedComponent :type Primitive%20Component%20Object%20Reference) (OtherActor :type Actor%20Object%20Reference) (OtherComp :type Primitive%20Component%20Object%20Reference) (OtherBodyIndex :type Integer) (bFromSweep :type Boolean) (SweepResult :type Hit%20Result%20Structure%20%28by%20ref%29))
  (bind _asittcharacter (Utilities|Casting|CastToITTCharacter OtherActor))
  (Utilities|FlowControl|Sequence
    (:then_0
      (Utilities|IsValid _asittcharacter
        (:Is%20Valid
          (Class|ITTCharacter|TakeDamage _asittcharacter 1.0 (Utilities|Struct|MakeDamageEvent) (Game|GetPlayerController 0) self)
          (Utilities|IsValid _asittcharacter
            (:Is%20Valid
              (Character|LaunchCharacter _asittcharacter "-200.000000, 0, 0" false false))))))))

(event OnComponentBeginOverlap(Left)
  (params (OverlappedComponent :type Primitive%20Component%20Object%20Reference) (OtherActor :type Actor%20Object%20Reference) (OtherComp :type Primitive%20Component%20Object%20Reference) (OtherBodyIndex :type Integer) (bFromSweep :type Boolean) (SweepResult :type Hit%20Result%20Structure%20%28by%20ref%29))
  (bind _asittcharacter (Utilities|Casting|CastToITTCharacter OtherActor))
  (Utilities|FlowControl|Sequence
    (:then_0
      (Utilities|IsValid _asittcharacter
        (:Is%20Valid
          (Class|ITTCharacter|TakeDamage _asittcharacter 1.0 (Utilities|Struct|MakeDamageEvent) (Game|GetPlayerController 0) self)
          (Utilities|IsValid _asittcharacter
            (:Is%20Valid
              (Character|LaunchCharacter _asittcharacter "-200.000000, 0, 0" false false))))))))

(event OnComponentBeginOverlap(BoomBox)
  (params (OverlappedComponent :type Primitive%20Component%20Object%20Reference) (OtherActor :type Actor%20Object%20Reference) (OtherComp :type Primitive%20Component%20Object%20Reference) (OtherBodyIndex :type Integer) (bFromSweep :type Boolean) (SweepResult :type Hit%20Result%20Structure%20%28by%20ref%29))
  (bind _asbp_fail_bomb (Utilities|Casting|CastToBP_FailBomb OtherActor))
  (if (not (Variables|/Game/GrabSystem/Blueprint/Actor/BP_Master_Grab.BP_Master_Grab_C|GetControllingByPlayer _asbp_fail_bomb))
    (Default|BombDestroy _asbp_fail_bomb)
    (Variables|Default|SetHealth (- (Variables|Default|GetHealth) 1e+01))))

(event Custom|clab
  (Animation|Montage|PlayMontage (Variables|Character|GetMesh) "/Game/Boss/calb+swing.calb+swing" 1.0 2.8))

(event Custom|swing
  (Animation|Montage|PlayMontage (Variables|Character|GetMesh) "/Game/Boss/swing.swing" 0.5))

(event Custom|RightHandStun
  (bind _output_get (Variables|Default|SetAttackIndex (+ (Variables|Default|GetAttackIndex) 1)))
  (bind _returnvalue (Game|SpawnActorfromClass "/Game/Boss/RHand.RHand_C" (Math|Transform|MakeTransform (Math|Vector|MakeVector (Math|Conversions|ToFloat(Integer) (Math|Random|RandomIntegerinRange -3400 -2300)) (Math|Conversions|ToFloat(Integer) (Math|Random|RandomIntegerinRange -1700 -600)) 3e+03) "0, 0, 0" "3.000000,3.000000,3.000000") "Undefined" 0 0))
  (bind _output_get_2 (Variables|/Game/Boss/RHand.RHand_C|SetAttackIndex _returnvalue _output_get))
  (bind _returnvalue_2 (Game|SpawnActorfromClass "/Game/Boss/DamegeAround.DamegeAround_C" (Math|Transform|MakeTransform (Math|Vector|MakeVector (.x (Transformation|GetActorLocation _returnvalue)) (.y (Transformation|GetActorLocation _returnvalue)) 1724.7501) "0, 0, 0" "10.000000,10.000000,10.000000") "Undefined" 0 0))
  (Variables|/Game/Boss/DamegeAround.DamegeAround_C|SetAttackIndex _returnvalue_2 _output_get_2))

(event Custom|ThrowBomb
  (bind _returnvalue (Game|SpawnActorfromClass "/Game/BossCreeper/BP_Bomb2.BP_Bomb2_C" (Math|Transform|MakeTransform (Math|Vector|MakeVector (Math|Conversions|ToFloat(Integer) (Math|Random|RandomIntegerinRange -3600 -2100)) (Math|Conversions|ToFloat(Integer) (Math|Random|RandomIntegerinRange -2000 1200)) 2.1e+03) "0, 0, 0" "1.000000,1.000000,1.000000") "Undefined" 0 0))
  (Rendering|Material|SetMaterial (Variables|/Script/Engine.Character|GetCapsuleComponent _returnvalue) 0 "/Game/BossCreeper/boom.boom"))

(event Custom|ThrowFailBomb
  (Game|SpawnActorfromClass "/Game/BossCreeper/BP_FailBomb.BP_FailBomb_C" (Math|Transform|MakeTransform (Math|Vector|MakeVector (Math|Conversions|ToFloat(Integer) (Math|Random|RandomIntegerinRange -3600 -2100)) (Math|Conversions|ToFloat(Integer) (Math|Random|RandomIntegerinRange -2000 1200)) 2.1e+03) "0, 0, 0" "1.000000,1.000000,1.000000") "Undefined" 0 0))

(event Custom|clab+swing
  (Animation|Montage|PlayMontage (Variables|Character|GetMesh) "/Game/Boss/calb+swing.calb+swing"))

(event Custom|LeftHandStun
  (bind _returnvalue (Game|SpawnActorfromClass "/Game/Boss/LHand.LHand_C" (Math|Transform|MakeTransform (Math|Vector|MakeVector (Math|Conversions|ToFloat(Integer) (Math|Random|RandomIntegerinRange -3400 -2300)) (Math|Conversions|ToFloat(Integer) (Math|Random|RandomIntegerinRange 0 900)) 3e+03) "0, 0, 0" "3.000000,3.000000,3.000000") "Undefined" 0 0))
  (Game|SpawnActorfromClass "/Game/Boss/DamegeAround.DamegeAround_C" (Math|Transform|MakeTransform (Math|Vector|MakeVector (.x (Transformation|GetActorLocation _returnvalue)) (.y (Transformation|GetActorLocation _returnvalue)) 1724.7501) "0, 0, 0" "10.000000,10.000000,10.000000") "Undefined" 0 0))

(event Custom|Phase1
  (Utilities|FlowControl|Delay 3.0)
  (switch int (Math|Random|RandomIntegerinRange 0 4)
    (:0
      (CallFunction|Swing)
      (CallFunction|Phase1))
    (:1
      (CallFunction|ThrowFailBomb)
      (CallFunction|Phase1))
    (:2
      (CallFunction|ThrowBomb)
      (CallFunction|Phase1))
    (:3
      (CallFunction|LeftHandStun)
      (CallFunction|Phase1))
    (:4
      (CallFunction|RightHandStun)
      (CallFunction|Phase1))))

(event EventBeginPlay
  (Variables|Default|SetHealth 1e+01)
  (Utilities|FlowControl|Delay 23.0)
  (bind _returnvalue (UserInterface|CreateWidget "/Game/Boss/UI_BossHPBar.UI_BossHPBar_C"))
  (UserInterface|Viewport|AddtoViewport _returnvalue 0)
  (CallFunction|Phase1))

(event EventTick
  (params (DeltaSeconds :type Float%20%28single-precision%29))
  (Utilities|FlowControl|Delay 1.1)
  (if (<= (Variables|Default|GetHealth) 0.0)
    (Animation|Montage|PlayMontage (Variables|Character|GetMesh) "/Game/Boss/BossDie.BossDie"
      (:OnCompleted
        (Game|OpenLevel(byName) "EndLevel")))))

(fn ConstructionScript)