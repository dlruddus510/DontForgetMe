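; BP_pressureplatform is a pressure plate that reacts when an ITTCharacter steps on or off it.
; On overlap it sphere-searches nearby SpawnPoint actors, spawns AppointBox at each, and plays a timeline that moves the Switch along Z.
; On exit it reverses the timeline and destroys newAppointBox, which holds only the last box spawned.
; If the search finds no spawn points, it prints a debug string.
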(event EventBeginPlay)

(event Collision|EventActorBeginOverlap
  (params (OtherActor :type Actor%20Object%20Reference))
  (Utilities|Casting|CastToITTCharacter OtherActor)
  (bind (_outactors _returnvalue) (Collision|SphereOverlapActors (Transformation|GetActorLocation) 2e+03 (Utilities|Array|MakeArray "ObjectTypeQuery2") "/Game/interactive/SpawnPoint.SpawnPoint_C"))
  (if _returnvalue
    (for _array_element _outactors
      (bind _returnvalue_2 (Game|SpawnActorfromClass "/Game/interactive/appointBox.appointBox_C" (Transformation|GetActorTransform _array_element) "Undefined" 0 0))
      (bind _switchposition (Timeline|SwitchActivate Play)
        (:Update
          (Transformation|SetRelativeLocation (Variables|Default|GetSwitch) (Math|Vector|MakeVector 0.0 0.0 _switchposition) false false))))
    (else
      (Development|PrintString "Hello"))))

(event EventTick
  (params (DeltaSeconds :type Float%20%28single-precision%29)))

(event Collision|EventActorEndOverlap
  (params (OtherActor :type Actor%20Object%20Reference))
  (Utilities|Casting|CastToITTCharacter OtherActor)
  (Actor|DestroyActor (stale Collision|EventActorBeginOverlap _returnvalue_2))
  (bind _switchposition (Timeline|SwitchActivate Reverse)
    (:Update
      (Transformation|SetRelativeLocation (Variables|Default|GetSwitch) (Math|Vector|MakeVector 0.0 0.0 _switchposition) false false))))

(fn ConstructionScript)