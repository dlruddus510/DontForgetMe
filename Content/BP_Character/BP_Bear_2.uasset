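; BP_Bear_2 is a bear character Blueprint that registers itself with the game instance when it spawns.
; On BeginPlay it casts to BP_GameInstance and appends itself to the SelectedCharacterBlueprint array.
; An unconnected chain, which never runs, would add itself and its skeletal mesh to Playeroption after a short delay in level1.
; Tick, overlap and the construction script are empty.
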(event Collision|EventActorBeginOverlap
  (params (OtherActor :type Actor%20Object%20Reference)))

(event EventTick
  (params (DeltaSeconds :type Float%20%28single-precision%29)))

(event EventBeginPlay
  (bind _asbp_game_instance (Utilities|Casting|CastToBP_GameInstance (Game|GetGameInstance)))
  (Utilities|Array|AppendArray (Variables|/Game/Blueprints/BP_GameInstance.BP_GameInstance_C|GetSelectedCharacterBlueprint _asbp_game_instance) (Utilities|Array|MakeArray self)))

(event Input|KeyboardEvents|LeftCtrl
  (params (Key :type Key%20Structure :default "None")))

(fn ConstructionScript)