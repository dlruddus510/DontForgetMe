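; Robot player character that fires a grappling-style hook and shows a respawn widget on request.
; Tick traces from the camera and swaps the robot's own mesh material when it hits a BP_Master_Grab actor.
; Primary action attaches a newly spawned rifle to the Grip socket, plays a montage, then after a delay spawns BP_Hook aimed by player-index-1 camera, with sound.
; Reset destroys the cable; cable-creation nodes are unconnected.
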(event Custom|OnFireProjectile)

(event Custom|Reset
  (bind _cable (Variables|Default|Getcable))
  (Utilities|FlowControl|Sequence
    (:then_0
      (Utilities|IsValid _cable
        (:Is%20Valid
          (Components|DestroyComponent _cable))))
    (:then_1
      (Utilities|FlowControl|DoOnce false) ; enters at Reset
    )))

(event EventBeginPlay
  (Variables|Default|SetSelectedCharacterType "Robot"))

(event Collision|EventActorBeginOverlap
  (params (OtherActor :type Actor%20Object%20Reference)))

(event EventPlayRespawnUI
  (bind _playerrespawn (Variables|Default|GetPlayerRespawn))
  (Class|UserWidget|SetPositioninViewport _playerrespawn (/ (* (Viewport|GetViewportSize) "(X=3.000000,Y=1.000000)") "(X=4.000000,Y=2.000000)") true)
  (UserInterface|Viewport|AddtoViewport _playerrespawn 0))

(event EventTick
  (params (DeltaSeconds :type Float%20%28single-precision%29))
  (bind _camera (Variables|Default|GetCamera))
  (bind _returnvalue (Transformation|GetWorldLocation _camera))
  (bind (_outhit _returnvalue_2) (Collision|LineTraceByChannel _returnvalue (+ _returnvalue (* (Math|Vector|GetForwardVector (Transformation|GetWorldRotation _camera)) 5e+03)) "TraceTypeQuery1" false 0 "None"))
  (Utilities|Casting|CastToBP_Master_Grab (.HitActor (Collision|BreakHitResult _outhit))
    (:then
      (if _returnvalue_2
        (Rendering|Material|SetMaterial (Variables|Character|GetMesh) 0 "/Game/Robot1/Material__89.Material__89")))
    (:CastFailed
      (Rendering|Material|SetMaterial (Variables|Character|GetMesh) 0 "/Game/Robot1/Material__47.Material__47"))))

(event Input|ActionEvents|InputActionPrimaryAction
  (params (Key :type Key%20Structure :default "None"))
  (bind _returnvalue (Game|GetPlayerCameraManager 1))
  (bind _projectileoffset (Variables|Default|GetProjectileOffset))
  (bind _mesh (Variables|Character|GetMesh))
  (bind _returnvalue_2 (Camera|GetCameraRotation _returnvalue))
  (bind _returnvalue_3 (Transformation|GetSocketLocation _mesh "Grip"))
  (bind _returnvalue_4 (Math|Vector|RotateVector _projectileoffset _returnvalue_2))
  (bind _returnvalue_5 (+ _returnvalue_3 _returnvalue_4))
  (:Pressed
    (Default|CallOnUseItem)
    (bind _returnvalue_6 (Game|SpawnActorfromClass "/Game/gungun/Blueprints/BP_Rifle.BP_Rifle_C" (Transformation|GetSocketTransform (Variables|Character|GetMesh) "Grip" "RTS_World") "Undefined" 0 0))
    (Transformation|AttachComponentToComponent _returnvalue_6 (Variables|Character|GetMesh) "Grip" "SnapToTarget" "SnapToTarget" "SnapToTarget" true)
    (Animation|Montage|MontagePlay (Components|SkeletalMesh|GetAnimInstance (Variables|Character|GetMesh)) "/Game/Robot1/anim/robot_hook1_Anim_M.robot_hook1_Anim_M" 0.2 "MontageLength" 0.0 true)
    (Utilities|FlowControl|Delay 1.5)
    (Game|SpawnActorfromClass "/Game/gungun/Blueprints/BP_Hook.BP_Hook_C" (Math|Transform|MakeTransform _returnvalue_5 _returnvalue_2) "Undefined" 0 0)
    (Audio|PlaySoundatLocation "/Game/FPWeapon/Audio/FirstPersonTemplateWeaponFire02.FirstPersonTemplateWeaponFire02" _returnvalue_5 "0, 0, 0" 1.0 1.0 0.0 0 0 0 0) ; Play firing sound
  ))

(event Input|TouchEvents|InputTouch
  (params (Location :type Vector) (FingerIndex :type ETouchIndex%20Enum))
  (:Pressed
    (if (Utilities|Enum|Equal(Enum) FingerIndex "Touch1") ; Only on first touch
      (Default|CallOnUseItem))))

(fn ConstructionScript)

(fn MakeCharacterTransparent
  (params (transparency :type Boolean))
  (bind _mesh (Variables|Character|GetMesh))
  (if true
    (Rendering|Material|SetMaterial _mesh 0 "/Game/Robot/1/Material__47.Material__47")
    (else
      (Rendering|Material|SetMaterial _mesh 0 "/Game/Robot1/Material__89.Material__89"))))