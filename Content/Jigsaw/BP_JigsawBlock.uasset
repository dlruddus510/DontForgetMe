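; BP_JigsawBlock is an actor for one jigsaw puzzle piece, shown as a static mesh with a coordinate-dependent material.
; StartCoordinate stores the given XY on the ACJigsawBlock component and calls its ChangeMaterial.
; It then applies the component's JigsawPiece material to the mesh's first slot.
; BeginPlay, Tick and construction only call the parent, so setup relies on StartCoordinate being called.
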(event EventBeginPlay
  (|CallParentFunction))

(event Collision|EventActorBeginOverlap
  (params (OtherActor :type Actor%20Object%20Reference)))

(event EventTick
  (params (DeltaSeconds :type Float%20%28single-precision%29))
  (|CallParentFunction DeltaSeconds))

(fn ConstructionScript
  (|CallParentFunction))

(fn StartCoordinate
  (params (XY :type Vector%202D%20Structure))
  (bind _ac_jigsawblock (Variables|Default|GetAC_JigsawBlock))
  (Variables|Default|SetXY (Math|Vector2D|MakeVector2D (.x XY) (.y XY)))
  (Variables|/Game/Jigsaw/AC_JigsawBlock.AC_JigsawBlock_C|SetPieceCoordinate _ac_jigsawblock (Math|Vector2D|MakeVector2D (.x XY) (.y XY)))
  (Default|ChangeMaterial _ac_jigsawblock)
  (Rendering|Material|SetMaterial (Variables|Default|GetStaticMesh) 0 (Variables|/Game/Jigsaw/AC_JigsawBlock.AC_JigsawBlock_C|GetJigsawPiece _ac_jigsawblock)))