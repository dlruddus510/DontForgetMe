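; AC_JigsawBlock represents one jigsaw puzzle piece and builds the material that shows its part of the puzzle image.
; ChangeMaterial creates a dynamic instance of Puzzle_mat_Inst and passes it the piece count, piece coordinate and image.
; The image's texture parameter name is None, and the SetMaterial node is unconnected, so the instance is never applied.
; BeginPlay and Tick are empty.
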(event EventBeginPlay)

(event EventTick
  (params (DeltaSeconds :type Float%20%28single-precision%29)))

(fn ChangeMaterial
  (bind _piececoordinate (Variables|Default|GetPieceCoordinate))
  (bind _returnvalue (Rendering|Material|CreateDynamicMaterialInstance "/Game/Image/Puzzle_mat_Inst.Puzzle_mat_Inst" "None" "None" :!class /Script/Engine.KismetMaterialLibrary))
  (bind _output_get (Variables|Default|SetJigsawPiece _returnvalue))
  (Rendering|Material|SetScalarParameterValue _output_get "Pieces" (Math|Conversions|ToFloat(Integer) (Variables|Default|GetNumberOfPieces)) :!class /Script/Engine.MaterialInstanceDynamic)
  (Rendering|Material|SetVectorParameterValue (Variables|Default|GetJigsawPiece) "PuzzleCoordinate" (Utilities|Struct|MakeLinearColor (.x _piececoordinate) (.y _piececoordinate) 0.0 0.0) :!class /Script/Engine.MaterialInstanceDynamic)
  (Rendering|Material|SetTextureParameterValue (Variables|Default|GetJigsawPiece) "None" (Variables|Default|GetJigsawImage)))