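; Jigsaw puzzle slot actor that catches an overlapping BP_JigsawBlock and records whether it is the correct piece.
; When empty, it snaps the block to its own transform, plays JigsawPuzzle and turns off the block's physics.
; It compares the block's image and coordinate to its own, then calls PuzzleCheck on the JigSaw_Board overlapping its Cube.
; A block ending overlap clears Installed but leaves CorrectBlock unchanged.
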(event Collision|EventActorBeginOverlap
  (params (OtherActor :type Actor%20Object%20Reference))
  (bind _asbp_jigsaw_block (Utilities|Casting|CastToBP_JigsawBlock OtherActor))
  (if (not (Variables|Default|GetbInstalled))
    (Variables|Default|SetbInstalled true)
    (Transformation|SetActorLocationAndRotation _asbp_jigsaw_block (Transformation|GetActorLocation) (Transformation|GetActorRotation))
    (Audio|Components|Audio|Play (Variables|Default|GetJigsaw_Puzzle) 0.0)
    (Physics|SetSimulatePhysics (Variables|/Game/GrabSystem/Blueprint/Actor/BP_Master_Grab.BP_Master_Grab_C|GetStaticMesh _asbp_jigsaw_block) false)
    (Variables|Default|SetbCorrectBlock (and (== (Variables|/Game/Jigsaw/BP_JigsawBlock.BP_JigsawBlock_C|GetImage _asbp_jigsaw_block) (Variables|Default|GetImage)) (Utilities|Operators|EqualEqual (Variables|/Game/Jigsaw/BP_JigsawBlock.BP_JigsawBlock_C|GetXY _asbp_jigsaw_block) (Variables|Default|GetCoordinate) 0.0)))
    (for _array_element (Collision|GetOverlappingActors (Variables|Default|GetCube) "/Game/Jigsaw/JigSaw_Board.JigSaw_Board_C" :!class /Script/Engine.PrimitiveComponent)
      _)
    (bind _asjig_saw_board (Utilities|Casting|CastToJigSaw_Board _array_element))
    (Default|PuzzleCheck _asjig_saw_board)))

(event Collision|EventActorEndOverlap
  (params (OtherActor :type Actor%20Object%20Reference))
  (Utilities|Casting|CastToBP_JigsawBlock OtherActor)
  (if (Variables|Default|GetbInstalled)
    (Variables|Default|SetbInstalled false)))

(fn ConstructionScript)