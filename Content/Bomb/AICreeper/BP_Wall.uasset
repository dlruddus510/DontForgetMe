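; BP_Wall is a wall actor in the bomb game's AICreeper folder that turns solid once something overlaps it.
; Its only live logic switches the StaticMesh collision response to Block on all channels at ActorBeginOverlap, with nothing active to revert it.
; Disconnected leftover nodes would restore Overlap, swap the mesh for a spawned actor plus a BP_ky_explosion, or destroy the wall, but never run.
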(event Collision|EventActorBeginOverlap
  (params (OtherActor :type Actor%20Object%20Reference))
  (Collision|SetCollisionResponsetoAllChannels (Variables|Default|GetStaticMesh) "ECR_Block"))

(fn ConstructionScript)