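; BP_FailBomb is a timed bomb actor that destroys itself and spawns an explosion effect three seconds after BeginPlay, dealing no damage.
; Two PawnSensing components set a seen-player flag and call FollowPlayer and FollowRobot, but both events are empty.
; Disconnected leftover nodes hold the unused AI chase, explosion and health-reduction logic for the Bear and Robot players.
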(event OnSeePawn(PawnSensing)
  (params (Pawn :type Pawn%20Object%20Reference))
  (Variables|Default|SetisSeeingPlayer? true)
  (CallFunction|FollowPlayer))

(event OnSeePawn(PawnSensing1)
  (params (Pawn :type Pawn%20Object%20Reference))
  (Variables|Default|SetisSeeingPlayer? true)
  (CallFunction|FollowRobot))

(event Custom|FollowPlayer)

(event Custom|FollowRobot)

(event Collision|EventActorBeginOverlap
  (params (OtherActor :type Actor%20Object%20Reference)))

(event EventBeginPlay
  (Utilities|FlowControl|Delay 3.0)
  (Actor|DestroyActor)
  (Effects|SpawnEmitteratLocation "/Game/FXVarietyPack/Particles/P_ky_explosion.P_ky_explosion" (Transformation|GetActorLocation)))

(fn ConstructionScript)