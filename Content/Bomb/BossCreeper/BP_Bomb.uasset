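; BP_Bomb is a self-destructing AI pawn that chases a player character and explodes.
; Two PawnSensing components set IsSeeingPlayer and trigger separate chases toward the BearCharacter (player 0) or Robot (player 1), regardless of which pawn was seen.
; AIMoveTo success destroys the bomb, spawns an explosion and subtracts one health from the target.
; Move failure does the same after a per-target delay, without checking distance.
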(event OnSeePawn(PawnSensing)
  (params (Pawn :type Pawn%20Object%20Reference))
  (Variables|Default|SetisSeeingPlayer? true)
  (CallFunction|FollowPlayer))

(event OnSeePawn(PawnSensing1)
  (params (Pawn :type Pawn%20Object%20Reference))
  (Variables|Default|SetisSeeingPlayer? true)
  (CallFunction|FollowRobot))

(event Custom|FollowPlayer
  (bind _asbear_character (Utilities|Casting|CastToBearCharacter (Game|GetPlayerCharacter 0)))
  (if (Variables|Default|GetisSeeingPlayer?)
    (AI|AIMoveTo self "0, 0, 0" _asbear_character 5.0 false
      (:OnSuccess
        (Actor|DestroyActor)
        (Effects|SpawnEmitteratLocation "/Game/FXVarietyPack/Particles/P_ky_explosion.P_ky_explosion" (Transformation|GetActorLocation))
        (Variables|/Script/DontForgetMe.ITTCharacter|SetCurrentHealth _asbear_character (- (Variables|/Script/DontForgetMe.ITTCharacter|GetCurrentHealth _asbear_character) 1.0)))
      (:OnFail
        (Utilities|FlowControl|Delay 1.0)
        (Actor|DestroyActor)
        (Effects|SpawnEmitteratLocation "/Game/FXVarietyPack/Particles/P_ky_explosion.P_ky_explosion" (Transformation|GetActorLocation))
        (Variables|/Script/DontForgetMe.ITTCharacter|SetCurrentHealth _asbear_character (- (Variables|/Script/DontForgetMe.ITTCharacter|GetCurrentHealth _asbear_character) 1.0))))))

(event Custom|FollowRobot
  (bind _asrobot (Utilities|Casting|CastToRobot (Game|GetPlayerCharacter 1)))
  (if (Variables|Default|GetisSeeingPlayer?)
    (AI|AIMoveTo self "0, 0, 0" _asrobot 5.0 false
      (:OnSuccess
        (Actor|DestroyActor)
        (Effects|SpawnEmitteratLocation "/Game/FXVarietyPack/Particles/P_ky_explosion.P_ky_explosion" (Transformation|GetActorLocation))
        (Variables|/Script/DontForgetMe.ITTCharacter|SetCurrentHealth _asrobot (- (Variables|/Script/DontForgetMe.ITTCharacter|GetCurrentHealth _asrobot) 1.0))
        (Development|PrintString (Utilities|String|ToString(Float) (- (Variables|/Script/DontForgetMe.ITTCharacter|GetCurrentHealth _asrobot) 1.0))))
      (:OnFail
        (Utilities|FlowControl|Delay 6.0)
        (Actor|DestroyActor)
        (Effects|SpawnEmitteratLocation "/Game/FXVarietyPack/Particles/P_ky_explosion.P_ky_explosion" (Transformation|GetActorLocation))
        (Variables|/Script/DontForgetMe.ITTCharacter|SetCurrentHealth _asrobot (- (Variables|/Script/DontForgetMe.ITTCharacter|GetCurrentHealth _asrobot) 1.0))
        (Development|PrintString (Utilities|String|ToString(Float) (- (Variables|/Script/DontForgetMe.ITTCharacter|GetCurrentHealth _asrobot) 1.0)))))))

(fn ConstructionScript)