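; BP_ThrowPuzzleManager is the manager actor for a throw puzzle that checks a six-color sequence against CorrectOrder.
; GetColorString collects unique colors, printing them until six are stored, then calls CheckPuzzleCompletion.
; A mismatch clears the sequence and calls OffMaterial on BP_Impactor and BP_Target actors tagged "TP".
; After the comparison loop, it disables the root component's tick and prints "good", even following a mismatch.
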(event EventBeginPlay)

(event Collision|EventActorBeginOverlap
  (params (OtherActor :type Actor%20Object%20Reference)))

(fn ConstructionScript)

(fn GetColorString
  (params (CS :type Enum_ImpactorColor%20Enum :default "NewEnumerator0"))
  (bind _colorstring (Variables|Default|GetColorString))
  (Utilities|Array|AddUnique _colorstring CS)
  (if (== (Utilities|Array|Length _colorstring) 6)
    (CallFunction|CheckPuzzleCompletion)
    (else
      (for _array_element (Variables|Default|GetColorString)
        (Development|PrintString (Utilities|String|EnumtoString _array_element))))))

(fn CheckPuzzleCompletion
  (bind _index (Utilities|FlowControl|ForLoopwithBreak 0 5)
    (:LoopBody
      (if (not (Utilities|Enum|Equal(Enum) (Utilities|Array|Get(acopy) (Variables|Default|GetCorrectOrder) _index) (Utilities|Array|Get(acopy) (Variables|Default|GetColorString) _index)))
        (Utilities|Array|Clear (Variables|Default|GetColorString))
        (bind _outactors (Actor|GetAllActorswithTag "TP"))
        (for _array_element _outactors
          (bind _asbp_impactor (Utilities|Casting|CastToBP_Impactor _array_element)
            (:then
              (Default|OffMaterial _asbp_impactor))
            (:CastFailed
              (bind _asbp_target (Utilities|Casting|CastToBP_Target _array_element))
              (Default|OffMaterial _asbp_target))))))
    (:Completed
      (Components|Tick|SetComponentTickEnabled (Variables|Default|GetDefaultSceneRoot) false)
      (Development|PrintString "good"))))