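; BP_Target is a target actor in the throw puzzle that tracks lit and success states and can launch colored impactors.
; SpawnImpactor spawns six scaled BP_Impactor actors at SpawnPoint, passing each the TPManager and a distinct color, then launches them along the Cube's right vector.
; The other functions only set the on/off and success flags or play the hit sound, with no event logic driving them here.
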(event EventBeginPlay)

(fn ConstructionScript)

(fn OffMaterial
  (Variables|Default|SetbisOn false))

(fn OnMaterial
  (Variables|Default|SetbisOn true))

(fn SpawnImpactor
  (for _index (range 0 5)
    (bind _returnvalue (Game|SpawnActorfromClass "/Game/ThrowPuzzle/BP_Impactor.BP_Impactor_C" (Math|Transform|MakeTransform (Transformation|GetWorldLocation (Variables|Default|GetSpawnPoint)) "0, 0, 0" "3.000000,3.000000,3.000000") "Undefined" 0 0))
    (Variables|/Game/ThrowPuzzle/BP_Impactor.BP_Impactor_C|SetTPManager _returnvalue (Variables|Default|GetTPManager))
    (Variables|/Game/ThrowPuzzle/BP_Impactor.BP_Impactor_C|SetColor _returnvalue (Utilities|Select :Index _index :Option%200 "NewEnumerator0" :Option%201 "NewEnumerator1" :Option%202 "NewEnumerator2" :Option%203 "NewEnumerator3" :Option%204 "NewEnumerator4" :Option%205 "NewEnumerator5"))
    (Default|SetMaterial _returnvalue)
    (Physics|SetPhysicsLinearVelocity (Variables|/Game/GrabSystem/Blueprint/Actor/BP_Master_Grab.BP_Master_Grab_C|GetStaticMesh _returnvalue) (* (Math|Vector|GetRightVector (Variables|Default|GetCube)) "600.000000,600.000000,600.000000") false "None")))

(fn StartSound
  (Audio|Components|Audio|Play (Variables|Default|Gettarget_hit) 0.0))

(fn PuzzleSuccess
  (Variables|Default|SetSuccess true))