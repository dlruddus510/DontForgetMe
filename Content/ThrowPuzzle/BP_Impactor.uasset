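; BP_Impactor is a color-coded throwable object for the throw puzzle that triggers BP_Target actors on contact.
; On BeginPlay it picks one of six cube materials from its Color value.
; When it overlaps a target while not player-controlled and not yet impacted, it starts the target's sound and material change, passes its color to TPManager's GetColorString, and destroys itself.
; Its own OnMaterial and OffMaterial functions only toggle the IsImpacted flag.
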(event EventBeginPlay
  (|CallParentFunction)
  (CallFunction|SetMaterial))

(event Collision|EventActorBeginOverlap
  (params (OtherActor :type Actor%20Object%20Reference))
  (bind _asbp_target (Utilities|Casting|CastToBP_Target OtherActor))
  (if (and (not (Variables|Default|GetControllingByPlayer)) (not (Variables|Default|GetisImpacted)))
    (Default|StartSound _asbp_target)
    (Default|OnMaterial _asbp_target)
    (CallFunction|OnMaterial)
    (Default|GetColorString (Variables|Default|GetTPManager) (Variables|Default|GetColor))
    (if (not (Variables|Default|GetControllingByPlayer))
      (Actor|DestroyActor))))

(event EventTick
  (params (DeltaSeconds :type Float%20%28single-precision%29))
  (|CallParentFunction DeltaSeconds) ; 지금 이 노드는 비활성 상태입니다. \n핀을 끌어서 다른 노드를 연결하면 활성화됩니다.
)

(fn ConstructionScript
  (|CallParentFunction))

(fn OnMaterial
  (Variables|Default|SetisImpacted true))

(fn OffMaterial
  (Variables|Default|SetisImpacted false))

(fn SetMaterial
  (Rendering|Material|SetMaterial (Variables|Default|GetStaticMesh) 0 (Utilities|Select :Index (Variables|Default|GetColor) :NewEnumerator0 "/Game/ThrowPuzzle/Red_cube_Mat.Red_cube_Mat" :NewEnumerator1 "/Game/ThrowPuzzle/Orange_cube_Mat.Orange_cube_Mat" :NewEnumerator2 "/Game/ThrowPuzzle/Yellow_cube_Mat.Yellow_cube_Mat" :NewEnumerator3 "/Game/ThrowPuzzle/Green_cube_Mat.Green_cube_Mat" :NewEnumerator4 "/Game/ThrowPuzzle/Blue_cube_Mat.Blue_cube_Mat" :NewEnumerator5 "/Game/ThrowPuzzle/Purple_cube_Mat.Purple_cube_Mat")))