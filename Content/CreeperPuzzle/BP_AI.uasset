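; BP_AI is a creeper-style suicide-bomber pawn in the CreeperPuzzle content that chases what it sees and explodes.
; PawnSensing feeds an AIMoveTo toward the seen pawn; on arrival, each overlapping ITTCharacter takes damage, and the pawn destroys itself with an explosion effect.
; Its own TakeDamage function returns zero without other logic.
; A delayed self-destruct chain is present but never runs.
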(event OnSeePawn(PawnSensing)
  (params (Pawn :type Pawn%20Object%20Reference))
  (AI|AIMoveTo self "0, 0, 0" Pawn 5.0 false
    (:OnSuccess
      (for _array_element (Collision|GetOverlappingActors "/Script/DontForgetMe.ITTCharacter" :!class /Script/Engine.Actor)
        (bind _asittcharacter (Utilities|Casting|CastToITTCharacter _array_element))
        (Class|ITTCharacter|TakeDamage _asittcharacter 1.0 (Utilities|Struct|MakeDamageEvent) (Pawn|GetController _asittcharacter) self)
        (Actor|DestroyActor)
        (Effects|SpawnEmitteratLocation "/Game/Realistic_Starter_VFX_Pack_Vol2/Particles/Explosion/P_Explosion_Big_A.P_Explosion_Big_A" (Transformation|GetActorLocation))))))

(fn ConstructionScript)

(fn TakeDamage
  (params (DamageAmount :type Float%20%28single-precision%29) (DamageEvent :type Damage%20Event%20Structure%20%28by%20ref%29) (EventInstigator :type Controller%20Object%20Reference) (DamageCauser :type Actor%20Object%20Reference))
  (return 0.0))