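; BP_Wall is a wall actor in the CreeperPuzzle folder that removes its mesh when any actor overlaps it.
; On overlap it sets the StaticMesh to block all channels, then destroys that component, leaving the actor itself in place.
; The hit event and construction script are empty.
; Disconnected leftover nodes for a cast, an overlap response, actor destruction and BP_KeyChild spawning never run.
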(event OnComponentHit(StaticMesh)
  (params (HitComponent :type Primitive%20Component%20Object%20Reference) (OtherActor :type Actor%20Object%20Reference) (OtherComp :type Primitive%20Component%20Object%20Reference) (NormalImpulse :type Vector :default "0, 0, 0") (Hit :type Hit%20Result%20Structure%20%28by%20ref%29)))

(event Collision|EventActorBeginOverlap
  (params (OtherActor :type Actor%20Object%20Reference))
  (Collision|SetCollisionResponsetoAllChannels (Variables|Default|GetStaticMesh) "ECR_Block")
  (Utilities|FlowControl|Sequence
    (:then_1
      (Components|DestroyComponent (Variables|Default|GetStaticMesh)))))

(fn ConstructionScript)